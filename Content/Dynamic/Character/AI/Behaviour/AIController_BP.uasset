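; AI controller for guard characters that starts the GuardBehaviour tree on the GuardData blackboard at BeginPlay.
; Perception updates set the blackboard Enemy key when an actor tagged Player is sensed.
; Any failed stimulus clears that key, whichever actor it came from.
; Helpers for writing stimulus and last-seen locations to the blackboard are defined but not called here.
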(event OnTargetPerceptionUpdated(AIPerception)
  (params (Actor :type Actor%20Object%20Reference) (Stimulus :type AI%20Stimulus%20Structure))
  (CallFunction|SetBlackboardEnemy Stimulus Actor))

(event EventBeginPlay
  (bind _blackboardcomponent (Class|AIController|UseBlackboard "/Game/Dynamic/Character/AI/Behaviour/GuardData.GuardData"))
  (Variables|Default|SetBlackboardCompRef _blackboardcomponent)
  (AI|RunBehaviorTree "/Game/Dynamic/Character/AI/Behaviour/GuardBehaviour.GuardBehaviour"))

(fn ConstructionScript)

(fn SetBlackboardEnemy
  (params (Stimulus :type AI%20Stimulus%20Structure) (Actor :type Actor%20Object%20Reference))
  (bind (_age _expirationage _strength _stimuluslocation _receiverlocation _tag _bsuccessfullysensed) (Utilities|Struct|BreakAIStimulus Stimulus))
  (LocalVariables|SetPerceived%20Actor Actor)
  (LocalVariables|SetStimulus%20Location _stimuluslocation)
  (if _bsuccessfullysensed
    (if (Actor|ActorHasTag Actor "Player")
      ;[1 1 1] Saw / Heard Player
      (CallFunction|SetEnemyonSight (Variables|Default|GetBlackboardCompRef) (LocalVariables|GetPerceived%20Actor)))
    (else
      ;[1 1 1] Not Stimulated
      (CallFunction|ClearEnemy (Variables|Default|GetBlackboardCompRef)))))

(fn ClearEnemy
  (params (Blackboard :type Blackboard%20Component%20Object%20Reference))
  (AI|Components|Blackboard|ClearValue Blackboard (Utilities|Name|MakeLiteralName "Enemy")))

(fn UpdateStimulusLocation
  (params (Blackboard :type Blackboard%20Component%20Object%20Reference) (Stimulus%20Location :type Vector))
  (AI|Components|Blackboard|SetValueasVector Blackboard (Utilities|Name|MakeLiteralName "StimulusLocation") Stimulus%20Location))

(fn SetEnemyonSight
  (params (Blackboard :type Blackboard%20Component%20Object%20Reference) (Perceived%20Actor :type Object%20Object%20Reference))
  (AI|Components|Blackboard|SetValueasObject Blackboard (Utilities|Name|MakeLiteralName "Enemy") Perceived%20Actor))

(fn UpdateEnemyLastSeenLocation
  (params (Blackboard :type Blackboard%20Component%20Object%20Reference) (Enemy%20Last%20Seen%20Location :type Vector))
  (AI|Components|Blackboard|SetValueasVector Blackboard (Utilities|Name|MakeLiteralName "EnemyLastSeenLocation") Enemy%20Last%20Seen%20Location))