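; BP_InfiniteTerrainGameMode is a game mode that builds chained terrain tiles and keeps a score.
; On BeginPlay it calls PopulateBoundsVolumePool, then spawns a few initial BP_Tile actors.
; SpawnTile places each tile at the stored SpawnTransform, then replaces it with the new tile's attach arrow transform so the next tile continues the chain.
; IncrementScore adds one to Score; neither it nor any further tile spawning is triggered within this Blueprint.
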(event EventBeginPlay
  (Class|InfiniteTerrainGameMode|PopulateBoundsVolumePool)
  (for _index (range 0 2)
    (CallFunction|SpawnTile)))

(event EventTick
  (params (DeltaSeconds :type Float%20%28single-precision%29)))

(fn ConstructionScript)

(fn SpawnTile
  (bind _returnvalue (Game|SpawnActorfromClass "/Game/Dynamic/Terrain/BP_Tile.BP_Tile_C" (Variables|Default|GetSpawn%20Transform) "Undefined" 0 0))
  (bind _attach_transform (Default|GetAttachArrowTransform _returnvalue))
  (Variables|Default|SetSpawn%20Transform _attach_transform))

(fn IncrementScore
  (Math|Integer|IncrementInt (Variables|Default|GetScore)))