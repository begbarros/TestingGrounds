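; Terrain tile for an infinite terrain mode that, on BeginPlay, locks its gate, scatters breakable boxes, takes the game mode's nav mesh bounds pool and places AI characters.
; A gate sensor unlocks the gate when the player enters; on exit it relocks it and has the game mode spawn another tile and increment score.
; A destroy sensor removes the tile on player overlap, and an arrow exposes the attach transform.
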(event OnComponentEndOverlap(GateSensor)
  (params (OverlappedComponent :type Primitive%20Component%20Object%20Reference) (OtherActor :type Actor%20Object%20Reference) (OtherComp :type Primitive%20Component%20Object%20Reference) (OtherBodyIndex :type Integer))
  (if (Utilities|IsActorPlayer OtherActor)
    (CallFunction|LockGate)
    (bind _asbp_infinite_terrain_game_mode (Utilities|Casting|CastToBP_InfiniteTerrainGameMode (Game|GetGameMode)))
    (Default|SpawnTile _asbp_infinite_terrain_game_mode)
    (Default|IncrementScore _asbp_infinite_terrain_game_mode)))

(event OnComponentBeginOverlap(GateDestroySensor)
  (params (OverlappedComponent :type Primitive%20Component%20Object%20Reference) (OtherActor :type Actor%20Object%20Reference) (OtherComp :type Primitive%20Component%20Object%20Reference) (OtherBodyIndex :type Integer) (bFromSweep :type Boolean) (SweepResult :type Hit%20Result%20Structure%20%28by%20ref%29))
  (if (Utilities|IsActorPlayer OtherActor)
    (Actor|DestroyActor)))

(event OnComponentBeginOverlap(GateSensor)
  (params (OverlappedComponent :type Primitive%20Component%20Object%20Reference) (OtherActor :type Actor%20Object%20Reference) (OtherComp :type Primitive%20Component%20Object%20Reference) (OtherBodyIndex :type Integer) (bFromSweep :type Boolean) (SweepResult :type Hit%20Result%20Structure%20%28by%20ref%29))
  (if (Utilities|IsActorPlayer OtherActor)
    (CallFunction|UnlockGate)))

(event EventBeginPlay
  (CallFunction|LockGate)
  (Class|Tile|PlaceActors "/Game/Props/BP_Breakable_Boxes.BP_Breakable_Boxes_C" 5e+02 50 100 1.0 2.0)
  (bind _asbp_infinite_terrain_game_mode (Utilities|Casting|CastToBP_InfiniteTerrainGameMode (Game|GetGameMode)))
  (Class|Tile|SetPool (Class|InfiniteTerrainGameMode|GetNavMeshBoundsVolumePool _asbp_infinite_terrain_game_mode))
  (Class|Tile|PlaceAI "/Game/Dynamic/Character/BP_Character.BP_Character_C" 5e+02 1 5))

(event Collision|EventActorBeginOverlap
  (params (OtherActor :type Actor%20Object%20Reference)))

(event EventTick
  (params (DeltaSeconds :type Float%20%28single-precision%29)))

(fn ConstructionScript)

(fn GetAttachArrowTransform
  (return (Transformation|GetWorldTransform (Variables|Default|GetArrow))))

(fn LockGate
  (Collision|SetCollisionEnabled (Variables|Default|GetGate) "QueryAndPhysics")
  (Rendering|Material|SetMaterial (Variables|Default|GetGate) 0 "/Game/Dynamic/Terrain/MI_GateLocked.MI_GateLocked"))

(fn UnlockGate
  (Collision|SetCollisionEnabled (Variables|Default|GetGate) "NoCollision")
  (Rendering|Material|SetMaterial (Variables|Default|GetGate) 0 "/Game/Dynamic/Terrain/MI_GateUnlocked.MI_GateUnlocked"))