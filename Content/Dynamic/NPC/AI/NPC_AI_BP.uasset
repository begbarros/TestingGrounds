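; NPC AI controller that runs a guard behavior tree and tracks the player as an enemy through AI perception.
; On BeginPlay it initializes the PatrolData blackboard, caches its component and starts GuardBehaviour.
; Perception updates write a sensed actor tagged Player to the Enemy key.
; Any failed-sense update clears that key, regardless of which actor triggered it.
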(event OnTargetPerceptionUpdated(AIPerception)
  (params (Actor :type Actor%20Object%20Reference) (Stimulus :type AI%20Stimulus%20Structure))
  (CallFunction|SetBlackboardEnemy Stimulus Actor))

(event EventBeginPlay
  (bind _blackboardcomponent (Class|AIController|UseBlackboard "/Game/Dynamic/NPC/AI/PatrolData.PatrolData"))
  (Variables|Default|SetBlackboardCompRef _blackboardcomponent)
  (AI|RunBehaviorTree "/Game/Dynamic/NPC/AI/GuardBehaviour.GuardBehaviour"))

(fn ConstructionScript)

(fn SetBlackboardEnemy
  (params (Stimulus :type AI%20Stimulus%20Structure) (Actor :type Actor%20Object%20Reference))
  (bind _returnvalue (Utilities|Name|MakeLiteralName "Enemy"))
  (bind _blackboardcompref (Variables|Default|GetBlackboardCompRef))
  (if (.bSuccessfullySensed (Utilities|Struct|BreakAIStimulus Stimulus))
    (if (Actor|ActorHasTag Actor "Player")
      (AI|Components|Blackboard|SetValueasObject _blackboardcompref _returnvalue Actor))
    (else
      (AI|Components|Blackboard|ClearValue _blackboardcompref _returnvalue))))